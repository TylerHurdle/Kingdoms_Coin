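; Left-side first coin platform in the Kingdoms coin game, which catches coins and spawns dropped ones.
; When the first found spawned coin overlaps its trigger, it marks platform 1 occupied on the hand spawner, destroys that coin and reveals a static dropped coin.
; SpawnLeftorRightCoin spawns a dropped coin randomly at the top left or right point.
; The bottom-spawn variant is uncalled here, and the switch overlap has no effect.
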(event OnComponentBeginOverlap(CoinOverlap(left))
  (params (OverlappedComponent :type Primitive%20Component%20Object%20Reference) (OtherActor :type Actor%20Object%20Reference) (OtherComp :type Primitive%20Component%20Object%20Reference) (OtherBodyIndex :type Integer) (bFromSweep :type Boolean) (SweepResult :type Hit%20Result%20Structure%20%28by%20ref%29))
  (bind _outactors (Actor|GetAllActorsOfClass "/Game/Character/bp_KingdomsCoinSpawnedCoin1.bp_KingdomsCoinSpawnedCoin1_C"))
  (if (Class|PrimitiveComponent|IsOverlappingComponent (Variables|/Game/Character/bp_KingdomsCoinSpawnedCoin1.bp_KingdomsCoinSpawnedCoin1_C|GetSphere (Utilities|Array|Get(acopy) _outactors)) OverlappedComponent)
    (bind _outactors_2 (Actor|GetAllActorsOfClass "/Game/Character/bp_KingdomsCoinHandSpawn.bp_KingdomsCoinHandSpawn_C"))
    (Variables|/Game/Character/bp_KingdomsCoinHandSpawn.bp_KingdomsCoinHandSpawn_C|SetIs%20Occupied%20on%20Platform1 (Utilities|Array|Get(acopy) _outactors_2) true)
    (Actor|DestroyActor (Utilities|Array|Get(acopy) _outactors))
    (Rendering|SetVisibility (Variables|Default|GetDroppedCoinLeft) true false)))

(event OnComponentBeginOverlap(CoinOverlap(leftswitch))
  (params (OverlappedComponent :type Primitive%20Component%20Object%20Reference) (OtherActor :type Actor%20Object%20Reference) (OtherComp :type Primitive%20Component%20Object%20Reference) (OtherBodyIndex :type Integer) (bFromSweep :type Boolean) (SweepResult :type Hit%20Result%20Structure%20%28by%20ref%29))
  (bind _outactors (Actor|GetAllActorsOfClass "/Game/Character/bp_KingdomsCoinSpawnedCoin1.bp_KingdomsCoinSpawnedCoin1_C"))
  (if (Class|PrimitiveComponent|IsOverlappingComponent (Variables|/Game/Character/bp_KingdomsCoinSpawnedCoin1.bp_KingdomsCoinSpawnedCoin1_C|GetSphere (Utilities|Array|Get(acopy) _outactors)))
    _))

(event Custom|Spawn%20Left%20or%20Right%20Coin
  (Utilities|ChooseLeftorRightCoin(top)))

(fn ConstructionScript)