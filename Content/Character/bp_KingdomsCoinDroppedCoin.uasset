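; Dropped coin actor for a Kingdoms coin platform setup, with a function that turns off physics on its sphere.
; Its DoOnce-gated conversion is meant to spawn a visible, scaled-down Platform1Right coin at Platform2's DoubleCoinOverlap, reset the gate and destroy itself.
; The overlap check that would trigger this is disconnected and the sphere's overlap event is empty, so the conversion never fires from this graph.
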(event OnComponentBeginOverlap(Sphere)
  (params (OverlappedComponent :type Primitive%20Component%20Object%20Reference) (OtherActor :type Actor%20Object%20Reference) (OtherComp :type Primitive%20Component%20Object%20Reference) (OtherBodyIndex :type Integer) (bFromSweep :type Boolean) (SweepResult :type Hit%20Result%20Structure%20%28by%20ref%29)))

(event Custom|reset
  (Utilities|FlowControl|DoOnce false) ; enters at Reset
)

(fn ConstructionScript)

(fn FStopSimulatingPhysics
  (Physics|SetSimulatePhysics (Variables|Default|GetSphere) false))