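; Spawned coin actor in the Kingdoms coin setup that reacts to the trigger zones of the left side of Platform 1.
; When its sphere begins an overlap inside CoinOverlapLeft, it has the platform spawn a left or right coin if the hand spawner reports Platform 1 occupied.
; Otherwise, it destroys itself if inside CoinOverlapLeftswitch.
; It finds platform and spawner through GetAllActorsOfClass, assuming one instance of each.
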(event OnComponentBeginOverlap(Sphere)
  (params (OverlappedComponent :type Primitive%20Component%20Object%20Reference) (OtherActor :type Actor%20Object%20Reference) (OtherComp :type Primitive%20Component%20Object%20Reference) (OtherBodyIndex :type Integer) (bFromSweep :type Boolean) (SweepResult :type Hit%20Result%20Structure%20%28by%20ref%29))
  (bind _outactors (Actor|GetAllActorsOfClass "/Game/Character/bp_KingdomsCoinPlatform1Left.bp_KingdomsCoinPlatform1Left_C"))
  (if (Class|PrimitiveComponent|IsOverlappingComponent (Variables|/Game/Character/bp_KingdomsCoinPlatform1Left.bp_KingdomsCoinPlatform1Left_C|GetCoinOverlap%28left%29 (Utilities|Array|Get(acopy) _outactors)) OverlappedComponent)
    (bind _outactors_2 (Actor|GetAllActorsOfClass "/Game/Character/bp_KingdomsCoinHandSpawn.bp_KingdomsCoinHandSpawn_C"))
    (if (Variables|/Game/Character/bp_KingdomsCoinHandSpawn.bp_KingdomsCoinHandSpawn_C|GetIs%20Occupied%20on%20Platform1 (Utilities|Array|Get(acopy) _outactors_2))
      (bind _outactors_3 (Actor|GetAllActorsOfClass "/Game/Character/bp_KingdomsCoinPlatform1Left.bp_KingdomsCoinPlatform1Left_C"))
      (Default|SpawnLeftorRightCoin (Utilities|Array|Get(acopy) _outactors_3)))
    (else
      (bind _outactors_4 (Actor|GetAllActorsOfClass "/Game/Character/bp_KingdomsCoinPlatform1Left.bp_KingdomsCoinPlatform1Left_C"))
      (if (Class|PrimitiveComponent|IsOverlappingComponent (Variables|/Game/Character/bp_KingdomsCoinPlatform1Left.bp_KingdomsCoinPlatform1Left_C|GetCoinOverlap%28leftswitch%29 (Utilities|Array|Get(acopy) _outactors_4)) OverlappedComponent)
        (Actor|DestroyActor)))))

(fn ConstructionScript)