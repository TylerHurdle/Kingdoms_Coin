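; Player controller for the Kingdoms Coin game that passes player input to the Player 1 hand actor.
; The move-right, move-left and spawn-coin actions each look up the first Bp_KingdomsCoinPlayer1Hand in the level and call its matching function.
; The hand is searched for on every press, and the construction script only assigns the HandReference variable to itself.
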(event EventBeginPlay)

(event EventTick
  (params (DeltaSeconds :type Float%20%28single-precision%29)))

(event Input|ActionEvents|InputActionMoveHandLeft
  (params (Key :type Key%20Structure :default "None"))
  (:Pressed
    (bind _outactors (Actor|GetAllActorsOfClass "/Game/Character/bp_KingdomsCoinPlayer1Hand.bp_KingdomsCoinPlayer1Hand_C"))
    (Default|FMoveHandLeft (Utilities|Array|Get(acopy) _outactors))))

(event Input|ActionEvents|InputActionMoveHandRight
  (params (Key :type Key%20Structure :default "None"))
  (:Pressed
    (bind _outactors (Actor|GetAllActorsOfClass "/Game/Character/bp_KingdomsCoinPlayer1Hand.bp_KingdomsCoinPlayer1Hand_C"))
    (Default|FMoveHandRight (Utilities|Array|Get(acopy) _outactors))))

(event Input|ActionEvents|InputActionSpawnCoin
  (params (Key :type Key%20Structure :default "None"))
  (:Pressed
    (bind _outactors (Actor|GetAllActorsOfClass "/Game/Character/bp_KingdomsCoinPlayer1Hand.bp_KingdomsCoinPlayer1Hand_C"))
    (Default|FSpawnCoin (Utilities|Array|Get(acopy) _outactors))))

(fn ConstructionScript
  (Variables|Default|SetHandReference (Variables|Default|GetHandReference)))